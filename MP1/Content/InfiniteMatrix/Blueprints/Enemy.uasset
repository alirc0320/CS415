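; Enemy actor that destroys itself three seconds after spawning or when its box overlaps a projectile or player.
; A player overlap subtracts 10 health, clamped between 0 and 100.
; A projectile overlap attempts to award score and update the score bar, but casts the projectile to BP_Player and uses the failed-cast branch, so the player reference is invalid.
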(event OnComponentBeginOverlap(Box)
  (params (OverlappedComponent :type Primitive%20Component%20Object%20Reference) (OtherActor :type Actor%20Object%20Reference) (OtherComp :type Primitive%20Component%20Object%20Reference) (OtherBodyIndex :type Integer) (bFromSweep :type Boolean) (SweepResult :type Hit%20Result%20Structure%20%28by%20ref%29))
  (Utilities|Casting|CastToBP_Projectile OtherActor
    (:then
      (Actor|DestroyActor)
      (Development|PrintString "DESTROYED!!!!!!!!")
      (bind _asbp_player (Utilities|Casting|CastToBP_Player OtherActor)
        (:CastFailed
          (Development|PrintString "Hello" true true "(R=0.000000,G=0.660000,B=1.000000,A=1.000000)" 1e+03)
          (bind _output_get (Variables|/Game/InfiniteMatrix/Blueprints/BP_Player.BP_Player_C|SetScore _asbp_player (+ (Variables|/Game/InfiniteMatrix/Blueprints/BP_Player.BP_Player_C|GetScore _asbp_player) 1e+03)))
          (Default|UpdateScore (Variables|/Game/InfiniteMatrix/Blueprints/BP_Player.BP_Player_C|GetOurScoreBar _asbp_player) _output_get)
          (Development|PrintString "GAINED POINTS!!!!!!!!!!!!"))))
    (:CastFailed
      (bind _asbp_player_2 (Utilities|Casting|CastToBP_Player OtherActor))
      (Variables|/Game/InfiniteMatrix/Blueprints/BP_Player.BP_Player_C|SetHealth _asbp_player_2 (Math|Float|Clamp(Float) (- (Variables|/Game/InfiniteMatrix/Blueprints/BP_Player.BP_Player_C|GetHealth _asbp_player_2) 1e+01) 0.0 1e+02))
      (Actor|DestroyActor))))

(event EventBeginPlay
  (Actor|GetAllActorsOfClass "Enemy_C")
  (Utilities|FlowControl|Delay 3.0)
  (Actor|DestroyActor)
  (Development|PrintString "enemy destoryed"))

(event Collision|EventActorBeginOverlap
  (params (OtherActor :type Actor%20Object%20Reference)))

(event EventTick
  (params (DeltaSeconds :type Float%20%28single-precision%29)))

(fn ConstructionScript)